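; VR player character driven by hand-pose gestures for locomotion and manipulation of VRTS_Pawn_Model actors.
; Each Tick polls both hands' pose recognizers, mapping pose indices to aiming at "move"-tagged surfaces, timeline-lerped XY movement, model selection and dragging.
; When both hands hold the scale pose, a camera sphere trace picks the model and hand-distance change resizes it.
; Enhanced Input drives per-hand widget clicks; SpaceBar logs encoded poses.
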(event `EnhancedInput|/Game/Input/LeftPressUI`
  (params (ActionValue :type Boolean) (ElapsedSeconds :type "Float (double-precision)") (TriggeredSeconds :type "Float (double-precision)") (InputAction :type "InputAction Object Reference" :default "/Game/Input/LeftPressUI.LeftPressUI"))
  (bind _leftwidgetinteraction (`self.LeftWidgetInteraction`))
  (:`Triggered`
    (if ActionValue :!label _label
      (`WidgetInteractionComponent.PressPointerKey` _leftwidgetinteraction "LeftMouseButton")
      (else
        (`WidgetInteractionComponent.ReleasePointerKey` _leftwidgetinteraction "LeftMouseButton" :!label _label_2))))
  (:`Started`
    (goto _label))
  (:`Ongoing`
    (goto _label))
  (:`Canceled`
    (goto _label_2))
  (:`Completed`
    (goto _label_2)))

(event `EnhancedInput|/Game/Input/RightPressUI`
  (params (ActionValue :type Boolean) (ElapsedSeconds :type "Float (double-precision)") (TriggeredSeconds :type "Float (double-precision)") (InputAction :type "InputAction Object Reference" :default "/Game/Input/RightPressUI.RightPressUI"))
  (bind _rightwidgetinteraction (`self.RightWidgetInteraction`))
  (:`Triggered`
    (if ActionValue :!label _label_3
      (`WidgetInteractionComponent.PressPointerKey` _rightwidgetinteraction "LeftMouseButton")
      (else
        (`WidgetInteractionComponent.ReleasePointerKey` _rightwidgetinteraction "LeftMouseButton" :!label _label_4))))
  (:`Started`
    (goto _label_3))
  (:`Ongoing`
    (goto _label_3))
  (:`Canceled`
    (goto _label_4))
  (:`Completed`
    (goto _label_4)))

(event `Key|SpaceBar`
  (params (Key :type "Key Structure"))
  (:`Pressed`
    (`HandPoseRecognizer.LogEncodedHandPose` (`self.LeftHandPoseRecognizer`))
    (`HandPoseRecognizer.LogEncodedHandPose` (`self.RightHandPoseRecognizer`))
    (`KismetSystemLibrary.PrintString` "pose loged" true true (struct :`R` 1.0 :`B` 0.118293 :`A` 1.0) 15.0)))

(event `self.ReceiveBeginPlay`
  (bind _returnvalue (pcsubsystem `EnhancedInputLocalPlayerSubsystem` (`GameplayStatics.GetPlayerController` 0)))
  (`HeadMountedDisplayFunctionLibrary.SetTrackingOrigin` "LocalFloor")
  (`/Engine/EditorBlueprintResources/StandardMacros.IsValid` _returnvalue
    (:`Is Valid`
      (`EnhancedInputSubsystemInterface.AddMappingContext` _returnvalue "/Game/Input/VRTSInputMappingContext.VRTSInputMappingContext" 0 (struct)))))

(event `Move`
  (params (`Is Left` :type Boolean))
  (bind (_current_location_x _current_location_y _current_location_z) (`KismetMathLibrary.BreakVector` (`self.current location`)))
  (bind _teleportvisualizerreference (`self.TeleportVisualizerReference`))
  (if (!= (`KismetMathLibrary.SelectVector` (`self.Left Hand Move Location`) (`self.Right Hand Move Location`) `Is Left`) (0.0 0.0 0.0))
    (set `self.Is Moving` true)
    (set `self.current location` (`self.K2_GetActorLocation`))
    (bind (_direction _alpha) (`Timeline|left hand` :!via `PlayFromStart`)
      (:`Update`
        (bind (_returnvalue_x _returnvalue_y) (`KismetMathLibrary.BreakVector` (`KismetMathLibrary.VLerp` (`self.current location`) (`KismetMathLibrary.SelectVector` (`self.Left Hand Move Location`) (`self.Right Hand Move Location`) `Is Left`) _alpha)))
        (`self.K2_SetActorLocation` (`KismetMathLibrary.MakeVector` _returnvalue_x _returnvalue_y _current_location_z)))
      (:`Finished`
        (set `self.Left Hand Move Location` (0.0 0.0 0.0))
        (set `self.Right Hand Move Location` (0.0 0.0 0.0))
        (`/Engine/EditorBlueprintResources/StandardMacros.IsValid` _teleportvisualizerreference
          (:`Is Valid`
            (`self.K2_DestroyActor` _teleportvisualizerreference))
          (:`Is Not Valid`
            _))
        (`KismetSystemLibrary.Delay` 0.25)
        (set `self.Is Moving` false)))))

(event `self.ReceiveTick`
  (params (DeltaSeconds :type "Float (single-precision)"))
  (bind _lefthand (`self.Lefthand`))
  (bind _righthand (`self.RightHand`))
  (`|ExecutionSequence`
    (:`then_0`
      (bind (_poseindex _posename) (`HandRecognitionFunctionLibrary.WaitForHandPose` (`self.LeftHandPoseRecognizer`))
        (:`PoseSeen`
          (switch `int` _poseindex
            (:`Default`
              (`self.Reset`))
            (:`0`
              (bind _location (`self.Move Scan` (`self.Lefthand`)))
              (set `self.Left Hand Move Location` _location)
              (set `self.Scale Left` false :!label _label_5)
              (set `self.Scale Right` false))
            (:`1`
              (`self.Move` true)
              (goto _label_5))
            (:`2`
              (if (not (`self.Right interacting`))
                (`self.Interact Scan` _lefthand)
                (goto _label_5)))
            (:`3`
              (`self.Move Model` _lefthand)
              (`KismetSystemLibrary.Delay` 6.0)
              (set `self.VRTS Model` null)
              (set `self.Left interacting` false)
              (goto _label_5))
            (:`4`
              (set `self.Scale Left` true))))))
    (:`then_1`
      (bind (_poseindex_2 _posename_2) (`HandRecognitionFunctionLibrary.WaitForHandPose` (`self.RightHandPoseRecognizer`))
        (:`PoseSeen`
          (switch `int` _poseindex_2
            (:`Default`
              (`self.Reset`))
            (:`0`
              (bind _location_2 (`self.Move Scan` (`self.RightHand`)))
              (set `self.Right Hand Move Location` _location_2)
              (set `self.Scale Left` false :!label _label_6)
              (set `self.Scale Right` false))
            (:`1`
              (`self.Move` false)
              (goto _label_6))
            (:`2`
              (if (not (`self.Left interacting`))
                (`self.Interact Scan` _righthand)
                (goto _label_6)))
            (:`3`
              (`self.Move Model` _righthand)
              (`KismetSystemLibrary.Delay` 6.0)
              (set `self.VRTS Model` null)
              (set `self.Right interacting` false)
              (goto _label_6))
            (:`4`
              (set `self.Scale Right` true))))))
    (:`then_2`
      (`self.Scale`)
      (`KismetSystemLibrary.Delay` 6.0)
      (set `self.Scale Right` false)
      (set `self.Scale Left` false)
      (set `self.VRTS Model` null)
      (set `self.Right interacting` false)
      (set `self.Left interacting` false))))

(event `Move Model`
  (params (`Target Hand` :type "OculusXRHandComponent Object Reference"))
  (bind _move_pivot (`self.Move Pivot`))
  (bind _vrts_model (`self.VRTS Model`))
  (`/Engine/EditorBlueprintResources/StandardMacros.IsValid` _vrts_model
    (:`Is Valid`
      (if (and (!= _move_pivot (0.0 0.0 0.0)) (`self.can move object `))
        (switch `EOculusXRHandType` (`OculusXRHandComponent.SkeletonType` `Target Hand`)
          (:`HandLeft`
            (set `self.Left interacting` true))
          (:`HandRight`
            (set `self.Right interacting` true)))
        (`self.K2_SetActorLocation` (`self.VRTS Model`) (+ (`self.K2_GetActorLocation` _vrts_model) (- (`SceneComponent.K2_GetComponentLocation` `Target Hand`) _move_pivot)) false false)
        (`KismetSystemLibrary.Delay` 1.0)
        (set `self.Move Pivot` (`SceneComponent.K2_GetComponentLocation` `Target Hand`))))))

(event `Scale`
  (bind _hand_distance (`self.Hand DIstance`))
  (bind _camera (`self.Camera`))
  (bind _returnvalue (`SceneComponent.K2_GetComponentLocation` _camera))
  (bind _returnvalue_2 (`KismetMathLibrary.Vector_Distance` (`SceneComponent.K2_GetComponentLocation` (`self.RightHand`)) (`SceneComponent.K2_GetComponentLocation` (`self.Lefthand`))))
  (if (and (`self.Scale Left`) (`self.Scale Right`))
    (`|ExecutionSequence`
      (:`then_0`
        (`/Engine/EditorBlueprintResources/StandardMacros.DoOnce` false :!label _label_7
          (:`Completed`
            (set `self.Hand DIstance` (`KismetMathLibrary.Vector_Distance` (`SceneComponent.K2_GetComponentLocation` (`self.RightHand`)) (`SceneComponent.K2_GetComponentLocation` (`self.Lefthand`)))))))
      (:`then_1`
        (set `self.Right interacting` true)
        (set `self.Left interacting` true)
        (bind _outhit (`KismetSystemLibrary.SphereTraceSingle` _returnvalue (+ _returnvalue (* (`SceneComponent.GetForwardVector` _camera) 750)) 10.0 "TraceTypeQuery1"))
        (bind _asvrts_pawn_model (cast `/Game/Blueprints/VRTS_Pawn_Model` (`.HitActor` (`GameplayStatics.BreakHitResult` _outhit))))
        (set `self.VRTS Model` _asvrts_pawn_model)
        (`self.SetActorScale3D` _asvrts_pawn_model (+ (`self.GetActorScale3D` _asvrts_pawn_model) (`KismetMathLibrary.SelectFloat` -0.01 (`KismetMathLibrary.SelectFloat` 0.01 0.0 (< _hand_distance _returnvalue_2)) (>= _hand_distance _returnvalue_2))))
        (`KismetSystemLibrary.Delay` 0.2)
        (set `self.Hand DIstance` (`KismetMathLibrary.Vector_Distance` (`SceneComponent.K2_GetComponentLocation` (`self.RightHand`)) (`SceneComponent.K2_GetComponentLocation` (`self.Lefthand`))))))
    (else
      (goto _label_7 :!via `Reset`))))

(fn `Hand Trace`
  (params (`Target Hand` :type "OculusXRHandComponent Object Reference") (Range :type Integer) (Radius :type "Float (single-precision)") (TraceChannel :type "ETraceTypeQuery Enum" :default "TraceTypeQuery1") (DrawDebugType :type "EDrawDebugTrace Enum" :default "None") (`Snap to ground` :type Boolean) (Offset :type "Vector Structure"))
  (returns (OutHit :type "HitResult Structure") (Hit :type Boolean))
  (bind _returnvalue (`SceneComponent.K2_GetComponentLocation` `Target Hand`))
  (bind (_returnvalue_x _returnvalue_y _returnvalue_z) (`KismetMathLibrary.BreakVector` (+ (* (`SceneComponent.GetUpVector` `Target Hand`) (select `EOculusXRHandType` (`OculusXRHandComponent.SkeletonType` `Target Hand`) :`HandLeft` Range :`HandRight` (* Range -1))) _returnvalue)))
  (bind (_outhit _returnvalue_2) (`KismetSystemLibrary.SphereTraceSingle` (+ _returnvalue Offset) (+ (`KismetMathLibrary.MakeVector` _returnvalue_x _returnvalue_y (`KismetMathLibrary.SelectFloat` 0.0 _returnvalue_z `Snap to ground`)) Offset) Radius TraceChannel false (`|MakeArray` self :!type "Actor Object Reference") DrawDebugType))
  (return _outhit _returnvalue_2))

(fn `Interact Scan`
  (params (`Target Hand` :type "OculusXRHandComponent Object Reference"))
  (bind _outhit (`self.Hand Trace` `Target Hand` 500 7.0 "TraceTypeQuery1" "None" false (0.0 0.0 10.0)))
  (bind _asvrts_pawn_model (cast `/Game/Blueprints/VRTS_Pawn_Model` (`.HitActor` (`GameplayStatics.BreakHitResult` _outhit)))
    (:`then`
      (set `self.VRTS Model` _asvrts_pawn_model)
      (set `self.Move Pivot` (`SceneComponent.K2_GetComponentLocation` `Target Hand`))
      (set `self.can move object ` true))
    (:`CastFailed`
      (set `self.VRTS Model` null)
      (set `self.Move Pivot` (0.0 0.0 0.0))
      (set `self.can move object ` false))))

(fn `Move Scan`
  (params (`Target Hand` :type "OculusXRHandComponent Object Reference"))
  (returns (Location :type "Vector Structure"))
  (bind _teleportvisualizerreference (`self.TeleportVisualizerReference`))
  (bind _teleportvisualizerreference_2 (`self.TeleportVisualizerReference`))
  (if (not (`self.Is Moving`))
    (bind _outhit (`self.Hand Trace` `Target Hand` 750 5.0 "TraceTypeQuery1" "None" true))
    (bind (_bblockinghit _binitialoverlap _time _distance _location _impactpoint _normal _impactnormal _physmat _hitactor) (`GameplayStatics.BreakHitResult` _outhit))
    (`/Engine/EditorBlueprintResources/StandardMacros.IsValid` _hitactor
      (:`Is Valid`
        (if (`self.ActorHasTag` _hitactor "move")
          (`/Engine/EditorBlueprintResources/StandardMacros.IsValid` _teleportvisualizerreference
            (:`Is Valid`
              (`self.K2_SetActorLocation` _teleportvisualizerreference _location false false)
              (return _location))
            (:`Is Not Valid`
              (bind _returnvalue (`|SpawnActorFromClass` "/Game/VRTemplate/Blueprints/VRTeleportVisualizer.VRTeleportVisualizer_C" (`KismetMathLibrary.MakeTransform` _location) "Undefined" "OverrideRootScale" self null))
              (set `self.TeleportVisualizerReference` _returnvalue)
              (return _location)))
          (else
            _)))
      (:`Is Not Valid`
        _))
    (return (0.0 0.0 0.0))
    (else
      (`/Engine/EditorBlueprintResources/StandardMacros.IsValid` _teleportvisualizerreference_2
        (:`Is Valid`
          (`self.K2_DestroyActor` _teleportvisualizerreference_2))))))

(fn `Reset`
  (bind _teleportvisualizerreference (`self.TeleportVisualizerReference`))
  (`/Engine/EditorBlueprintResources/StandardMacros.IsValid` _teleportvisualizerreference
    (:`Is Valid`
      (`self.K2_DestroyActor` _teleportvisualizerreference))
    (:`Is Not Valid`
      _))
  (set `self.Left interacting` false)
  (set `self.Scale Left` false)
  (set `self.Scale Right` false)
  (set `self.VRTS Model` null)
  (set `self.Move Pivot` (0.0 0.0 0.0)))

(fn `UserConstructionScript`)